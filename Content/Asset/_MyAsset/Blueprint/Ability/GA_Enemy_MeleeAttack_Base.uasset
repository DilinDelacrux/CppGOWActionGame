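; Base gameplay ability for enemy melee attacks: plays an attack montage and applies damage when a hit lands.
; On activation it plays the montage and waits for a Shared.Event.MeleeHit gameplay event while it runs.
; Each hit applies a shared damage effect spec, scaled by a configurable scalable float, to the event target, then fires a weapon hit sound gameplay cue on success.
; The ability ends when the montage completes, blends out, or is interrupted or cancelled.
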(event `self.K2_ActivateAbility`
  (`AbilityTask_PlayMontageAndWait.CreatePlayMontageAndWaitProxy` "None" (`self.Montage to Play`)
    (:`then`
      (bind (_asynctaskproxy _payload) (`AbilityTask_WaitGameplayEvent.WaitGameplayEvent` (struct :`TagName` "Shared.Event.MeleeHit") null)
        (:`EventReceived`
          (`self.Handle Apply Damage` _payload))))
    (:`OnCompleted`
      (`self.K2_EndAbility` :!label _label))
    (:`OnBlendOut`
      (goto _label))
    (:`OnInterrupted`
      (goto _label))
    (:`OnCancelled`
      (goto _label))))

(fn `Handle Apply Damage`
  (params (InPayload :type "GameplayEventData Structure"))
  (`self.BP_ApplyEffectSpecHandleToTarget` (`.Target` (break `GameplayEventData` InPayload)) (`self.MakeEnemyDamageEffectSpecHandle` "/Game/Asset/_MyAsset/GameEffect/GE_Shared_DealDamage.GE_Shared_DealDamage_C" (`self.In Damage Scalable Float`))
    (:`Successful`
      (`self.K2_ExecuteGameplayCue` (`self.WeaponHitSoundGameCueTag`)))))