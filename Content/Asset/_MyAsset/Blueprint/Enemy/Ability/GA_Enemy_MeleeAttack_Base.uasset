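; Base enemy melee attack ability that plays an attack montage and applies damage when a melee hit event arrives.
; Enemies tagged Unblockable first fire a warning gameplay cue.
; Hit events apply a damage effect spec to the target; on success, a weapon hit sound cue plays and a hit-react event is sent to that target.
; The ability ends when the montage completes, blends out, is interrupted or is cancelled.
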(event `self.K2_ActivateAbility`
  (`WarriorFunctionLibrary.BP_DoesActorHaveTag` (`self.GetEnemyCharacterFromActorInfo`) (struct :`TagName` "Enemy.Status.Unblockable")
    (:`YES`
      (`self.K2_ExecuteGameplayCueWithParams` (struct :`TagName` "GameplayCue.FX.Unblockable.Warning") (`AbilitySystemBlueprintLibrary.MakeGameplayCueParameters` 0.0 (`self.UnblockableWarningSpawnedDistance`)))
      (`KismetSystemLibrary.Delay` 0.2))
    (:`NO`
      _))
  (`AbilityTask_PlayMontageAndWait.CreatePlayMontageAndWaitProxy` "None" (`self.Montage to Play`)
    (:`then`
      (bind (_asynctaskproxy _payload) (`AbilityTask_WaitGameplayEvent.WaitGameplayEvent` (struct :`TagName` "Shared.Event.MeleeHit") null)
        (:`EventReceived`
          (`self.Handle Apply Damage` _payload))))
    (:`OnCompleted`
      (`self.K2_EndAbility` :!label _label))
    (:`OnBlendOut`
      (goto _label))
    (:`OnInterrupted`
      (goto _label))
    (:`OnCancelled`
      (goto _label))))

(fn `Handle Apply Damage`
  (params (InPayload :type "GameplayEventData Structure"))
  (bind (_eventtag _instigator _target) (break `GameplayEventData` InPayload))
  (`self.BP_ApplyEffectSpecHandleToTarget` _target (`self.MakeEnemyDamageEffectSpecHandle` "/Game/Asset/_MyAsset/GameEffect/GE_Shared_DealDamage.GE_Shared_DealDamage_C" (`self.In Damage Scalable Float`))
    (:`Successful`
      (`|ExecutionSequence`
        (:`then_0`
          (`self.K2_ExecuteGameplayCue` (`self.WeaponHitSoundGameCueTag`)))
        (:`then_1`
          (`AbilitySystemBlueprintLibrary.SendGameplayEventToActor` _target (struct :`TagName` "Shared.Event.HitReact") (`local.InPayload`)))))))