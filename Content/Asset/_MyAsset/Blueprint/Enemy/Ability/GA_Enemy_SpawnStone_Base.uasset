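; Base enemy gameplay ability that gives a level-scaled chance to spawn a healing or rage stone near the enemy.
; On activation it traces down from the enemy and picks a random navigable point around the impact.
; If the weighted roll passes, it picks either stone class at random, async loads it and spawns it there with random yaw.
; Debug prints report progress, with the printed roll evaluated separately from the branch's roll.
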(event `self.K2_ActivateAbility`
  (bind _returnvalue (`self.GetEnemyCharacterFromActorInfo`))
  (bind _returnvalue_2 (`Actor.K2_GetActorLocation` _returnvalue))
  (bind _returnvalue_3 (`WarriorFunctionLibrary.GetScalableFloatValueAtLevel` (`self.SpawnChance`) (`KismetMathLibrary.Conv_IntToDouble` (`self.GetAbilityLevel`))))
  (bind _returnvalue_4 (`KismetMathLibrary.RandomBoolWithWeight` _returnvalue_3))
  (`|ExecutionSequence`
    (:`then_0`
      (bind _outhit (`KismetSystemLibrary.LineTraceSingleForObjects` _returnvalue_2 (+ (* (`Actor.GetActorUpVector` _returnvalue) -200.0) _returnvalue_2) (`self.Object Types`)))
      (bind (_randomlocation _returnvalue_5) (`NavigationSystemV1.K2_GetRandomLocationInNavigableRadius` (`.ImpactPoint` (`GameplayStatics.BreakHitResult` _outhit)) 200.0 null null))
      (if _returnvalue_5
        (set `self.RandomSpawnLocation` _randomlocation)
        (else
          (`self.K2_EndAbility`))))
    (:`then_1`
      (`KismetSystemLibrary.PrintString` (`KismetTextLibrary.Conv_TextToString` (`|FormatText` "Spawn chance = {0} spawn or not ={1}" _returnvalue_3 _returnvalue_4)) true true (struct :`R` 1.0 :`G` 0.039932 :`A` 1.0) 5.0)
      (if _returnvalue_4
        (if (`KismetMathLibrary.RandomBool`)
          (set `self.StoneClassToSpawn` "/Game/Asset/_MyAsset/Blueprint/Items/Stones/BP_Stone_HealingStone.BP_Stone_HealingStone_C")
          (else
            (set `self.StoneClassToSpawn` "/Game/Asset/_MyAsset/Blueprint/Items/Stones/BP_Stone_RageStone.BP_Stone_RageStone_C")))
        (bind _class (`|LoadAssetClass` (`self.StoneClassToSpawn`))
          (:`then`
            (`KismetSystemLibrary.PrintString` "Start Async load" true true (struct :`R` 1.0 :`G` 0.039932 :`A` 1.0) 5.0))
          (:`Completed`
            (`KismetSystemLibrary.PrintString` "Async load Complete" true true (struct :`R` 1.0 :`G` 0.039932 :`A` 1.0) 5.0)
            (bind _asactor (castclass `Actor` _class)
              (:`then`
                (`|SpawnActorFromClass` _asactor (`KismetMathLibrary.MakeTransform` (`self.RandomSpawnLocation`) (`KismetMathLibrary.MakeRotator` 0.0 0.0 (`KismetMathLibrary.RandomFloatInRange` 0.0 359.0))) "AdjustIfPossibleButAlwaysSpawn" "MultiplyWithRoot" null null)
                (`KismetSystemLibrary.PrintString` "Spawn Stone" true true (struct :`R` 1.0 :`G` 0.039932 :`A` 1.0) 5.0)
                (`self.K2_EndAbility`))
              (:`CastFailed`
                (`KismetSystemLibrary.PrintString` "Cast Failed " true true (struct :`R` 1.0 :`G` 0.039932 :`A` 1.0) 5.0)
                (`self.K2_EndAbility`)))))
        (else
          (`self.K2_EndAbility`))))))