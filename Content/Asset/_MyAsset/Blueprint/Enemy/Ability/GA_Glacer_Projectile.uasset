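; Gameplay ability for the Glacer enemy that casts a projectile.
; Activation plays the Gruntling cast montage and then waits for the Shared.Event.SpawnProjectile gameplay event.
; On that event it spawns BP_Projectile_Glacer at the ProjectileSpawnSocket, aimed along the enemy's forward vector and carrying a damage effect spec built from a scalable float.
; The ability ends when the montage completes, blends out, is interrupted or is cancelled.
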(event `self.K2_ActivateAbility`
  (bind _returnvalue (`self.GetEnemyCharacterFromActorInfo`))
  (`AbilityTask_PlayMontageAndWait.CreatePlayMontageAndWaitProxy` "None" "/Game/Asset/_MyAsset/Animation/Montage/Enemy/Guardian/AM_ExoGame_Gruntling_Cast.AM_ExoGame_Gruntling_Cast"
    (:`then`
      (`AbilityTask_WaitGameplayEvent.WaitGameplayEvent` (struct :`TagName` "Shared.Event.SpawnProjectile") null
        (:`EventReceived`
          (`|SpawnActorFromClass` "/Game/Asset/_MyAsset/Blueprint/Enemy/Glacer/BP_Projectile_Glacer.BP_Projectile_Glacer_C" (`KismetMathLibrary.MakeTransform` (`SceneComponent.GetSocketLocation` (`self.GetOwningComponentFromActorInfo`) "ProjectileSpawnSocket") (`KismetMathLibrary.Conv_VectorToRotator` (`Actor.GetActorForwardVector` _returnvalue))) "Undefined" "MultiplyWithRoot" _returnvalue (`self.MakeEnemyDamageEffectSpecHandle` "/Game/Asset/_MyAsset/GameEffect/GE_Shared_DealDamage.GE_Shared_DealDamage_C" (`self.ProjectileDamageScalableFloat`)) _returnvalue))))
    (:`OnCompleted`
      (`self.K2_EndAbility` :!label _label))
    (:`OnBlendOut`
      (goto _label))
    (:`OnInterrupted`
      (goto _label))
    (:`OnCancelled`
      (goto _label))))