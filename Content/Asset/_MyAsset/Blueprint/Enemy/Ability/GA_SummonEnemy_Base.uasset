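; Base gameplay ability for enemies that summons other enemies while playing a montage.
; Once the montage starts, a WaitSpawnEnemies task listens for the summon event tag and spawns the configured count of a soft-referenced class around the enemy's location.
; When spawning finishes it sets the HasSpawnEnemies blackboard bool.
; The ability ends on any montage exit: completion, blend out, interruption or cancellation.
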(event `self.K2_ActivateAbility`
  (`AbilityTask_PlayMontageAndWait.CreatePlayMontageAndWaitProxy` "None" (`self.Montage to Play`)
    (:`then`
      (`AbilityTask_WaitSpawnEnemies.WaitSpawnEnemies` (struct :`TagName` "Enemy.Event.SummonEnemies") (`self.Soft Enemy Class to Spawn`) (`self.Num to Spawn`) (`Actor.K2_GetActorLocation` (`self.GetEnemyCharacterFromActorInfo`))
        (:`OnSpawnFinished`
          (`BlackboardComponent.SetValueAsBool` (`AIBlueprintHelperLibrary.GetBlackboard` (`self.GetEnemyCharacterFromActorInfo`)) "HasSpawnEnemies" true))))
    (:`OnCompleted`
      (`self.K2_EndAbility` :!label _label))
    (:`OnBlendOut`
      (goto _label))
    (:`OnInterrupted`
      (goto _label))
    (:`OnCancelled`
      (goto _label))))