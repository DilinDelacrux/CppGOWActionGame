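; Hero block ability that holds a standing block montage with a magic shield cue until interrupted or cancelled.
; Successful block events turn the hero toward the attacker, apply root-motion knockback and fire an impact cue.
; Blocks landing within the threshold after activation count as perfect, adding a cue, brief global slow motion and a timed JumpToFinisher tag.
; Ending the ability restores normal time dilation.
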(event `self.K2_ActivateAbility`
  (set `self.HeroBlockActivatedTime` (`GameplayStatics.GetTimeSeconds`))
  (`AbilityTask_PlayMontageAndWait.CreatePlayMontageAndWaitProxy` "None" "/Game/Asset/_MyAsset/Animation/Montage/Hero/AM_Hero_StandingBlock_Idle.AM_Hero_StandingBlock_Idle"
    (:`then`
      (`|ExecutionSequence`
        (:`then_0`
          (`self.K2_AddGameplayCueWithParams` (struct :`TagName` "GameplayCue.FX.MagicShield") (`AbilitySystemBlueprintLibrary.MakeGameplayCueParameters` 0.0 0.0 (struct) (struct) (struct) (struct) (struct) (0.0 0.0 0.0) (0.0 0.0 0.0) null null null null 1 (`self.GetAbilityLevel`) (`self.GetOwningComponentFromActorInfo`))))
        (:`then_1`
          (bind (_asynctaskproxy _payload) (`AbilityTask_WaitGameplayEvent.WaitGameplayEvent` (struct :`TagName` "Player.Event.SuccessfulBlock") null)
            (:`EventReceived`
              (`|ExecutionSequence`
                (:`then_0`
                  (set `self.IsPerfectBlock` (<= (- (`GameplayStatics.GetTimeSeconds`) (`self.HeroBlockActivatedTime`)) (`self.PerfectBlockThreshold`)))
                  (`Actor.K2_SetActorRotation` (`self.GetHeroCharacterFromActorInfo`) (`KismetMathLibrary.FindLookAtRotation` (`Actor.K2_GetActorLocation` (`self.GetHeroCharacterFromActorInfo`)) (`Actor.K2_GetActorLocation` (`.Instigator` (break `GameplayEventData` _payload)))) false))
                (:`then_1`
                  (`AbilityTask_ApplyRootMotionConstantForce.ApplyRootMotionConstantForce` "None" (`KismetMathLibrary.NegateVector` (`Actor.GetActorForwardVector` (`self.GetHeroCharacterFromActorInfo`))) 80.0 0.2 false "/MeshModelingToolsetExp/Curves/ContrastAdjustmentCurve.ContrastAdjustmentCurve" "MaintainLastRootMotionVelocity"))
                (:`then_2`
                  (`self.K2_ExecuteGameplayCueWithParams` (struct :`TagName` "GameplayCue.FX.MagicShield.SuccessfullyBlock") (`self.MakeBlockGameplayParams`)))
                (:`then_3`
                  (if (`self.IsPerfectBlock`)
                    (`WarriorFunctionLibrary.AddGameplayTagToActorIfNone` (`self.GetHeroCharacterFromActorInfo`) (struct :`TagName` "Player.Status.JumpToFinisher"))
                    (`self.K2_ExecuteGameplayCueWithParams` (struct :`TagName` "GameplayCue.FX.MagicShield.PerfectBlock") (`self.MakeBlockGameplayParams`))
                    (`GameplayStatics.SetGlobalTimeDilation` 0.2)
                    (`KismetSystemLibrary.Delay` 0.08)
                    (`GameplayStatics.SetGlobalTimeDilation` 1.0)
                    (`self.StartResetJumpToFinishTimer`)))))))))
    (:`OnInterrupted`
      (`self.K2_EndAbility` :!label _label)
      (`self.StartResetJumpToFinishTimer`))
    (:`OnCancelled`
      (goto _label))))

(event `self.K2_OnEndAbility`
  (params (bWasCancelled :type Boolean))
  (if (!= (`GameplayStatics.GetGlobalTimeDilation`) 1.0)
    (`GameplayStatics.SetGlobalTimeDilation` 1.0)))

(event `StartResetJumpToFinishTimer`
  (`KismetSystemLibrary.K2_SetTimerDelegate` (delegate `ResetJumpToFinishState`) (`self.PerfectBlockParryWindow`)))

(event `ResetJumpToFinishState`
  (`WarriorFunctionLibrary.RemoveGameplayTagToActorIfFound` (`self.GetHeroCharacterFromActorInfo`) (struct :`TagName` "Player.Status.JumpToFinisher")))

(fn `MakeBlockGameplayParams`
  (returns (ReturnValue :type "GameplayCueParameters Structure"))
  (return (`AbilitySystemBlueprintLibrary.MakeGameplayCueParameters` 0.0 0.0 (struct) (struct) (struct) (struct) (struct) (0.0 0.0 0.0) (0.0 0.0 0.0) null null null null 1 1 (`self.GetOwningComponentFromActorInfo`))))