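; Gameplay ability that plays the hero's hit reaction when activated by a gameplay event.
; It computes a direction tag from the instigator and the hero, then switches on it to pick a front, left, right or back montage, defaulting to front.
; It sets a hit FX material parameter once the montage starts and clears it when the ability ends, which follows montage completion, blend out, interruption or cancellation.
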(event `self.K2_ActivateAbilityFromEvent`
  (params (EventData :type "GameplayEventData Structure (by ref)"))
  (`|SwitchGameplayTag` (`.ReturnValue` (`WarriorFunctionLibrary.ComputeHitReactDirectionTag` (`.Instigator` (break `GameplayEventData` EventData)) (`self.GetHeroCharacterFromActorInfo`)))
    (:`Default`
      (set `self.Montage to Play` "/Game/Asset/_MyAsset/Animation/Montage/Hero/HitReact/AM_Hero_HitReactLarge_Front.AM_Hero_HitReactLarge_Front" :!label _label))
    (:`Shared.Status.HitReact.Front`
      (goto _label))
    (:`Shared.Status.HitReact.Left`
      (set `self.Montage to Play` "/Game/Asset/_MyAsset/Animation/Montage/Hero/HitReact/AM_Hero_HitReactLarge_Left.AM_Hero_HitReactLarge_Left"))
    (:`Shared.Status.HitReact.Right`
      (set `self.Montage to Play` "/Game/Asset/_MyAsset/Animation/Montage/Hero/HitReact/AM_Hero_HitReact_Right.AM_Hero_HitReact_Right"))
    (:`Shared.Status.HitReact.Back`
      (set `self.Montage to Play` "/Game/Asset/_MyAsset/Animation/Montage/Hero/HitReact/AM_Hero_HitReact_Back.AM_Hero_HitReact_Back")))
  (`AbilityTask_PlayMontageAndWait.CreatePlayMontageAndWaitProxy` "None" (`self.Montage to Play`)
    (:`then`
      (`MeshComponent.SetScalarParameterValueOnMaterials` (`self.GetOwningComponentFromActorInfo`) "HitFxSwitch" 1.0))
    (:`OnCompleted`
      (`self.K2_EndAbility` :!label _label_2))
    (:`OnBlendOut`
      (goto _label_2))
    (:`OnInterrupted`
      (goto _label_2))
    (:`OnCancelled`
      (goto _label_2))))

(event `self.K2_OnEndAbility`
  (params (bWasCancelled :type Boolean))
  (`MeshComponent.SetScalarParameterValueOnMaterials` (`self.GetOwningComponentFromActorInfo`) "HitFxSwitch" 0.0))