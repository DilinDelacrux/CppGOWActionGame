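; Hero gameplay ability for Rage mode, entered with an axe shout montage and an Activating status tag that clears when the montage ends.
; A montage-time gameplay event adds the rage cue, which lasts until the ability ends.
; A rage cost effect runs while the ability stays active beyond the montage.
; The Rage.None tag cancels the ability, and ending it removes the cost effect by its stored handle.
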(event `self.K2_ActivateAbility`
  (`WarriorFunctionLibrary.AddGameplayTagToActorIfNone` (`self.GetHeroCharacterFromActorInfo`) (struct :`TagName` "Player.Status.Rage.Activating"))
  (`AbilityTask_PlayMontageAndWait.CreatePlayMontageAndWaitProxy` "None" "/Game/Asset/_MyAsset/Animation/Montage/Hero/AM_Hero_Axe_Shout_Adjusted.AM_Hero_Axe_Shout_Adjusted"
    (:`then`
      (`|ExecutionSequence`
        (:`then_0`
          (`AbilityTask_WaitGameplayEvent.WaitGameplayEvent` (struct :`TagName` "Player.Event.ActivateRage") null
            (:`EventReceived`
              (`self.K2_AddGameplayCueWithParams` (struct :`TagName` "GameplayCue.FX.Rage.Activating") (`AbilitySystemBlueprintLibrary.MakeGameplayCueParameters` 0.0 0.0 (struct) (struct) (struct) (struct) (struct) (0.0 0.0 0.0) (0.0 0.0 0.0) null null null null 1 1 (`self.GetOwningComponentFromActorInfo`))))))
        (:`then_1`
          (`AbilityTask_WaitGameplayTagAdded.WaitGameplayTagAdd` (struct :`TagName` "Player.Status.Rage.None") null
            (:`Added`
              (`self.K2_CancelAbility`))))
        (:`then_2`
          (bind _returnvalue (`self.BP_ApplyGameplayEffectToOwner` "/Game/Asset/_MyAsset/GameEffect/GE_Hero_Cost_Rage.GE_Hero_Cost_Rage_C" (`self.GetAbilityLevel`)))
          (set `self.AppliedRageCostGameplayEffectHandle` _returnvalue))))
    (:`OnCompleted`
      (`WarriorFunctionLibrary.RemoveGameplayTagToActorIfFound` (`self.GetHeroCharacterFromActorInfo`) (struct :`TagName` "Player.Status.Rage.Activating") :!label _label))
    (:`OnBlendOut`
      (goto _label))
    (:`OnInterrupted`
      (goto _label))
    (:`OnCancelled`
      (goto _label))))

(event `self.K2_OnEndAbility`
  (params (bWasCancelled :type Boolean))
  (`self.BP_RemoveGameplayEffectFromOwnerWithHandle` (`self.AppliedRageCostGameplayEffectHandle`)))