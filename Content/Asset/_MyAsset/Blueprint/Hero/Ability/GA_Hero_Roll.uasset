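; Gameplay ability that performs the hero's dodge roll in the direction of last movement input.
; After a brief delay so input is valid, it sets motion warp targets for roll direction and a landing point traced down to the ground at a level-scaled distance.
; It then plays the roll montage, adding a ForceFocusingTarget status tag that is removed when the ability ends.
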(event `self.K2_ActivateAbility`
  ;[1 1 1] 保证有Last movement input vector
  (`KismetSystemLibrary.Delay` 0.05)
  (`self.ComputeRollDirectionAndDistance`)
  (`AbilityTask_PlayMontageAndWait.CreatePlayMontageAndWaitProxy` "None" "/Game/Asset/_MyAsset/Animation/Montage/Hero/AM_Hero_Roll.AM_Hero_Roll"
    (:`then`
      (`WarriorFunctionLibrary.AddGameplayTagToActorIfNone` (`self.GetHeroCharacterFromActorInfo`) (struct :`TagName` "Player.Status.ForceFocusingTarget")))
    (:`OnCompleted`
      (`self.K2_EndAbility` :!label _label))
    (:`OnBlendOut`
      (goto _label))
    (:`OnInterrupted`
      (goto _label))
    (:`OnCancelled`
      (goto _label))))

(event `self.K2_OnEndAbility`
  (params (bWasCancelled :type Boolean))
  (`WarriorFunctionLibrary.RemoveGameplayTagToActorIfFound` (`self.GetHeroCharacterFromActorInfo`) (struct :`TagName` "Player.Status.ForceFocusingTarget")))

(fn `ComputeRollDirectionAndDistance`
  (locals (CachedRollingDirection :type "Vector Structure" :default (0.0 0.0 0.0)))
  (bind _returnvalue (`Actor.K2_GetActorLocation` (`self.GetHeroCharacterFromActorInfo`)))
  (bind _motionwarpingcomponent (`WarriorBaseCharacter.MotionWarpingComponent` (`self.GetHeroCharacterFromActorInfo`)))
  (bind _returnvalue_2 (+ (`Actor.K2_GetActorLocation` (`self.GetHeroCharacterFromActorInfo`)) (* (`local.CachedRollingDirection`) (`WarriorFunctionLibrary.GetScalableFloatValueAtLevel` (`self.RollingDistanceScalableFloat`) (`KismetMathLibrary.Conv_IntToDouble` (`self.GetAbilityLevel`))))))
  (bind _output_get (set `local.CachedRollingDirection` (`KismetMathLibrary.Normal` (`Pawn.GetLastMovementInputVector` (`self.GetHeroCharacterFromActorInfo`)))))
  (`KismetSystemLibrary.DrawDebugArrow` _returnvalue (+ _returnvalue (* _output_get 200.0)) 50.0 (struct :`R` 1.0 :`B` 0.184016 :`A` 1.0) 20.0 5.0)
  (`|ExecutionSequence`
    (:`then_0`
      (`MotionWarpingComponent.AddOrUpdateWarpTargetFromLocationAndRotation` (`WarriorBaseCharacter.MotionWarpingComponent` (`self.GetHeroCharacterFromActorInfo`)) "RollingDirection" (0.0 0.0 0.0) (`KismetMathLibrary.MakeRotFromX` (`local.CachedRollingDirection`))))
    (:`then_1`
      (bind _outhit (`KismetSystemLibrary.LineTraceSingleForObjects` _returnvalue_2 (+ _returnvalue_2 (* (`KismetMathLibrary.NegateVector` (`Actor.GetActorUpVector` (`self.GetHeroCharacterFromActorInfo`))) 500.0)) (`self.Object Types`)))
      (bind (_bblockinghit _binitialoverlap _time _distance _location _impactpoint) (`GameplayStatics.BreakHitResult` _outhit))
      (if _bblockinghit
        (`MotionWarpingComponent.AddOrUpdateWarpTargetFromLocation` _motionwarpingcomponent "RollingTargetLocation" _impactpoint)
        (else
          (`MotionWarpingComponent.RemoveWarpTarget` _motionwarpingcomponent "RollingTargetLocation"))))))