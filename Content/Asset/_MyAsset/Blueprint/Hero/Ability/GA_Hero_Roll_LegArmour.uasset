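; Hero gameplay ability for the LegArmour roll, which can also damage enemies through melee hit events.
; After a brief delay for movement input, it picks a back or side montage from input versus facing.
; Motion warping targets set roll rotation and a ground-traced landing point.
; It adds a force-focus tag until ability end; hits apply light-attack weapon damage, trigger hit reacts and grant rage.
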(event `self.K2_ActivateAbility`
  (`KismetSystemLibrary.PrintString` "LegArmour")
  ;[1 1 1] 保证有Last movement input vector
  (`KismetSystemLibrary.Delay` 0.05)
  (`self.ComputeRollDirectionAndDistance`)
  (`AbilityTask_PlayMontageAndWait.CreatePlayMontageAndWaitProxy` "None" (`self.Montage to Play`)
    (:`then`
      (`WarriorFunctionLibrary.AddGameplayTagToActorIfNone` (`self.GetHeroCharacterFromActorInfo`) (struct :`TagName` "Player.Status.ForceFocusingTarget"))
      (bind (_asynctaskproxy _payload) (`AbilityTask_WaitGameplayEvent.WaitGameplayEvent` (struct :`TagName` "Shared.Event.MeleeHit") null)
        (:`EventReceived`
          (`self.HandleApplyDamage` _payload))))
    (:`OnCompleted`
      (`self.K2_EndAbility` :!label _label))
    (:`OnBlendOut`
      (goto _label))
    (:`OnInterrupted`
      (goto _label))
    (:`OnCancelled`
      (goto _label))))

(event `self.K2_OnEndAbility`
  (params (bWasCancelled :type Boolean))
  (`WarriorFunctionLibrary.RemoveGameplayTagToActorIfFound` (`self.GetHeroCharacterFromActorInfo`) (struct :`TagName` "Player.Status.ForceFocusingTarget")))

(fn `ComputeRollDirectionAndDistance`
  (locals (CachedRollingDirection :type "Vector Structure" :default (0.0 0.0 0.0)))
  (bind _motionwarpingcomponent (`WarriorBaseCharacter.MotionWarpingComponent` (`self.GetHeroCharacterFromActorInfo`)))
  (bind _returnvalue (+ (`Actor.K2_GetActorLocation` (`self.GetHeroCharacterFromActorInfo`)) (* (`local.CachedRollingDirection`) (select `bool` (`self.bRollBack`) :`false` 300.0 :`true` 200.0))))
  (bind _output_get (set `local.CachedRollingDirection` (`KismetMathLibrary.Normal` (`Pawn.GetLastMovementInputVector` (`self.GetHeroCharacterFromActorInfo`)))))
  (bind _output_get_2 (set `self.bRollBack` (< (`KismetMathLibrary.Dot_VectorVector` _output_get (`Actor.GetActorForwardVector` (`self.GetHeroCharacterFromActorInfo`))) (`self.Roll Back Threshold`))))
  (set `self.Montage to Play` (select `bool` _output_get_2 :`false` "/Game/Asset/_MyAsset/Animation/Montage/Hero/BareHand/AM_Hero_LegArmour_RollSide.AM_Hero_LegArmour_RollSide" :`true` "/Game/Asset/_MyAsset/Animation/Montage/Hero/BareHand/AM_Hero_LegArmour_RollBack.AM_Hero_LegArmour_RollBack" :!type "AnimMontage Object Reference"))
  (`|ExecutionSequence`
    (:`then_0`
      (`MotionWarpingComponent.AddOrUpdateWarpTargetFromLocationAndRotation` (`WarriorBaseCharacter.MotionWarpingComponent` (`self.GetHeroCharacterFromActorInfo`)) "RollingDirection" (0.0 0.0 0.0) (`KismetMathLibrary.ComposeRotators` (`KismetMathLibrary.MakeRotFromX` (`local.CachedRollingDirection`)) (select `bool` (`self.bRollBack`) :`false` (struct :`Yaw` 90.0) :`true` (struct :`Yaw` 180.0) :!type "Rotator Structure"))))
    (:`then_1`
      (bind _outhit (`KismetSystemLibrary.LineTraceSingleForObjects` _returnvalue (+ _returnvalue (* (`KismetMathLibrary.NegateVector` (`Actor.GetActorUpVector` (`self.GetHeroCharacterFromActorInfo`))) 500.0)) (`self.Object Types`)))
      (bind (_bblockinghit _binitialoverlap _time _distance _location _impactpoint) (`GameplayStatics.BreakHitResult` _outhit))
      (if _bblockinghit
        (`MotionWarpingComponent.AddOrUpdateWarpTargetFromLocation` _motionwarpingcomponent "RollingTargetLocation" _impactpoint)
        (else
          (`MotionWarpingComponent.RemoveWarpTarget` _motionwarpingcomponent "RollingTargetLocation"))))))

(fn `HandleApplyDamage`
  (params (GameplayEventData :type "GameplayEventData Structure (by ref)"))
  (bind (_eventtag _instigator _target) (break `GameplayEventData` GameplayEventData))
  (`self.K2_ExecuteGameplayCue` (`self.WeaponHitSoundGameplayCueTag`))
  (`self.BP_ApplyEffectSpecHandleToTarget` _target (`self.MakeHeroDamageEffectSpecHandle` "/Game/Asset/_MyAsset/GameEffect/GE_Shared_DealDamage.GE_Shared_DealDamage_C" (`HeroCombatComponent.GetHeroCurrentEquipWeaponDamageAtLevel` (`self.GetHeroCombatComponent`) (`KismetMathLibrary.Conv_IntToDouble` (`self.GetAbilityLevel`))) (struct :`TagName` "Player.SetByCaller.AttackType.Light"))
    (:`Successful`
      (`AbilitySystemBlueprintLibrary.SendGameplayEventToActor` _target (struct :`TagName` "Shared.Event.HitReact") (`local.GameplayEventData`))
      (`self.BP_ApplyGameplayEffectToOwner` "/Game/Asset/_MyAsset/GameEffect/GE_Hero_GainRage.GE_Hero_GainRage_C" (`self.GetAbilityLevel`))
      (return))))