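; Hero gameplay ability for the axe's heavy special attack, a jump attack with area damage.
; Activation plays the montage, then commits the ability and notifies the hero UI of the cooldown.
; On the Player.Event.AOE gameplay event, a box trace around and ahead of the hero applies weapon-based damage, scaled by ability level, to the hits.
; The ability ends when the montage completes, blends out or is stopped.
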(event `self.K2_ActivateAbility`
  (bind _returnvalue (`self.GetCooldownTimeRemaining`))
  (bind _returnvalue_2 (`self.GetHeroCharacterFromActorInfo`))
  (bind _returnvalue_3 (`Actor.K2_GetActorLocation` _returnvalue_2))
  (bind _returnvalue_4 (`Actor.GetActorForwardVector` _returnvalue_2))
  (bind (_heroweapondata_weaponanimlayertolink _heroweapondata_defaultweaponabilities _heroweapondata_specialweaponabilities _heroweapondata_weaponinputmappingcontext _heroweapondata_weaponbasedamage) (break `WarriorHeroWeaponData` (`WarriorHeroWeapon.HeroWeaponData` (`HeroCombatComponent.GetHeroCurrentEquipWeapon` (`self.GetHeroCombatComponent`)))))
  (`AbilityTask_PlayMontageAndWait.CreatePlayMontageAndWaitProxy` "None" "/Game/Asset/_MyAsset/Animation/Montage/Hero/AM_Hero_Axe_JumpAttack.AM_Hero_Axe_JumpAttack"
    (:`then`
      (`|ExecutionSequence`
        (:`then_0`
          (`AbilityTask_WaitGameplayEvent.WaitGameplayEvent` (struct :`TagName` "Player.Event.AOE") null
            (:`EventReceived`
              (bind _outhits (`KismetSystemLibrary.BoxTraceMultiForObjects` _returnvalue_3 (+ _returnvalue_3 (* _returnvalue_4 200.0)) (500.0 500.0 200.0) (`KismetMathLibrary.Conv_VectorToRotator` _returnvalue_4) (`self.Object Types`)))
              (`self.ApplyGameplayEffectSpecHandleToHitResults` (`self.MakeHeroDamageEffectSpecHandle` "/Game/Asset/_MyAsset/GameEffect/GE_Shared_DealDamage.GE_Shared_DealDamage_C" (`WarriorFunctionLibrary.GetScalableFloatValueAtLevel` _heroweapondata_weaponbasedamage (`KismetMathLibrary.Conv_IntToDouble` (`self.GetAbilityLevel`))) (struct :`TagName` "InputTag.SpecialWeaponAbility.Heavy") 3) _outhits))))
        (:`then_1`
          (`self.K2_CommitAbility`)
          (`HeroUIComponent.OnAbilityCooldownBegin` (`WarriorHeroCharacter.HeroUIComponent` (`self.GetHeroCharacterFromActorInfo`)) (struct :`TagName` "InputTag.SpecialWeaponAbility.Heavy") _returnvalue _returnvalue))))
    (:`OnCompleted`
      (`self.K2_EndAbility` :!label _label))
    (:`OnBlendOut`
      (goto _label))
    (:`OnInterrupted`
      (goto _label))
    (:`OnCancelled`
      (goto _label))))