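; Hero gameplay ability for the axe's light special attack, a strike that deals damage and sets the target burning.
; It plays the attack montage, commits, signals the cooldown to the hero UI, and ends when the montage finishes or is interrupted.
; Melee-hit events apply level-scaled damage, then send a hit react and apply a tagged fire damage-over-time effect.
; A successful burn grants the hero rage.
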(event `self.K2_ActivateAbility`
  (bind _returnvalue (`self.GetCooldownTimeRemaining`))
  (`AbilityTask_PlayMontageAndWait.CreatePlayMontageAndWaitProxy` "None" "/Game/Asset/_MyAsset/Animation/Montage/Hero/Attack/AM_Hero_Axe_Ability_Light.AM_Hero_Axe_Ability_Light"
    (:`then`
      (`|ExecutionSequence`
        (:`then_0`
          (bind (_asynctaskproxy _payload) (`AbilityTask_WaitGameplayEvent.WaitGameplayEvent` (struct :`TagName` "Shared.Event.MeleeHit") null)
            (:`EventReceived`
              (`self.HandleApplyDamage` _payload))))
        (:`then_1`
          (`self.K2_CommitAbility`)
          (`HeroUIComponent.OnAbilityCooldownBegin` (`WarriorHeroCharacter.HeroUIComponent` (`self.GetHeroCharacterFromActorInfo`)) (struct :`TagName` "InputTag.SpecialWeaponAbility.Light") _returnvalue _returnvalue))))
    (:`OnCompleted`
      (`self.K2_EndAbility` :!label _label))
    (:`OnBlendOut`
      (goto _label))
    (:`OnInterrupted`
      (goto _label))
    (:`OnCancelled`
      (goto _label))))

(fn `HandleApplyDamage`
  (params (GameplayEventData :type "GameplayEventData Structure (by ref)"))
  (bind (_eventtag _instigator _target) (break `GameplayEventData` GameplayEventData))
  (`self.K2_ExecuteGameplayCue` (`self.WeaponHitSoundGameplayCueTag`))
  (`self.BP_ApplyEffectSpecHandleToTarget` _target (`self.MakeHeroDamageEffectSpecHandle` "/Game/Asset/_MyAsset/GameEffect/GE_Shared_DealDamage.GE_Shared_DealDamage_C" (`WarriorFunctionLibrary.GetScalableFloatValueAtLevel` (`self.StartDamage`) (`KismetMathLibrary.Conv_IntToDouble` (`self.GetAbilityLevel`))) (struct :`TagName` "Player.SetByCaller.AttackType.Light") 1)
    (:`Successful`
      (`AbilitySystemBlueprintLibrary.SendGameplayEventToActor` _target (struct :`TagName` "Shared.Event.HitReact") (`local.GameplayEventData`))
      (`WarriorFunctionLibrary.AddGameplayTagToActorIfNone` _target (struct :`TagName` "Shared.Status.Burning"))
      (`self.BP_ApplyEffectSpecHandleToTarget` _target (`self.MakeHeroStatusEffectSpecHandle` "/Game/Asset/_MyAsset/GameEffect/GE_Shared_BurningDamage.GE_Shared_BurningDamage_C" (`WarriorFunctionLibrary.GetScalableFloatValueAtLevel` (`self.BurningDamage`) (`KismetMathLibrary.Conv_IntToDouble` (`self.GetAbilityLevel`))) (struct :`TagName` "Player.SetByCaller.AttackType.Status") (struct :`TagName` "Shared.DamageType.Fire") 0 0 (`WarriorFunctionLibrary.GetScalableFloatValueAtLevel` (`self.BurningDuration`) (`KismetMathLibrary.Conv_IntToDouble` (`self.GetAbilityLevel`))))
        (:`Successful`
          (`self.BP_ApplyGameplayEffectToOwner` "/Game/Asset/_MyAsset/GameEffect/GE_Hero_GainRage.GE_Hero_GainRage_C" (`self.GetAbilityLevel`))
          (return))
        (:`Failed`
          (return))))
    (:`Failed`
      (return))))