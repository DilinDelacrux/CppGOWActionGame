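; Hero gameplay ability for the leg armour's light special attack: a motion-warped montage strike with a cooldown shown in the UI.
; A forward box trace sets the warp target to the closest hit actor, or a point ahead, with debug spheres; ending removes it.
; Melee hit events apply damage, then hit react, a Burning tag and a timed status effect that is actually Ice damage.
; Successful status application grants the hero rage.
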(event `self.K2_ActivateAbility`
  (bind _returnvalue (`self.GetCooldownTimeRemaining`))
  (`self.ComputeMotionWarping`)
  (`AbilityTask_PlayMontageAndWait.CreatePlayMontageAndWaitProxy` "None" "/Game/Asset/_MyAsset/Animation/Montage/Hero/BareHand/AM_Hero_LegArmour_SpecialAbility_Light.AM_Hero_LegArmour_SpecialAbility_Light"
    (:`then`
      (`|ExecutionSequence`
        (:`then_0`
          (bind (_asynctaskproxy _payload) (`AbilityTask_WaitGameplayEvent.WaitGameplayEvent` (struct :`TagName` "Shared.Event.MeleeHit") null)
            (:`EventReceived`
              (`self.HandleApplyDamage` _payload))))
        (:`then_1`
          (`self.K2_CommitAbility`)
          (`HeroUIComponent.OnAbilityCooldownBegin` (`WarriorHeroCharacter.HeroUIComponent` (`self.GetHeroCharacterFromActorInfo`)) (struct :`TagName` "InputTag.SpecialWeaponAbility.Light") _returnvalue _returnvalue))))
    (:`OnCompleted`
      (`self.K2_EndAbility` :!label _label))
    (:`OnBlendOut`
      (goto _label))
    (:`OnInterrupted`
      (goto _label))
    (:`OnCancelled`
      (goto _label))))

(event `self.K2_OnEndAbility`
  (params (bWasCancelled :type Boolean))
  (`MotionWarpingComponent.RemoveWarpTarget` (`WarriorBaseCharacter.MotionWarpingComponent` (`self.GetHeroCharacterFromActorInfo`)) "WarpLocation"))

(fn `ComputeMotionWarping`
  (locals (HalfSizeX :type "Float (double-precision)" :default 700.0))
  (bind _returnvalue (`self.GetHeroCharacterFromActorInfo`))
  (bind _returnvalue_2 (`self.GetHeroCharacterFromActorInfo`))
  (bind _returnvalue_3 (`Actor.K2_GetActorLocation` _returnvalue_2))
  (bind _returnvalue_4 (`Actor.GetActorForwardVector` _returnvalue_2))
  (bind _motionwarpingcomponent (`WarriorBaseCharacter.MotionWarpingComponent` (`self.GetHeroCharacterFromActorInfo`)))
  (bind _returnvalue_5 (+ (`Actor.K2_GetActorLocation` _returnvalue) (* (`Actor.GetActorForwardVector` _returnvalue) 500.0)))
  (bind _outhits (`KismetSystemLibrary.BoxTraceMultiForObjects` _returnvalue_3 (+ _returnvalue_3 (* _returnvalue_4 200.0)) (500.0 500.0 200.0) (`KismetMathLibrary.Conv_VectorToRotator` _returnvalue_4) (`self.Object Types`)))
  (bind (_outclosesthit _returnvalue_6) (`WarriorFunctionLibrary.FindClosestHitIgnoreActors` _outhits (`|MakeArray` _returnvalue :!type "Actor Object Reference")))
  (if _returnvalue_6
    (bind _returnvalue_7 (`Actor.K2_GetActorLocation` (`.HitActor` (`GameplayStatics.BreakHitResult` _outclosesthit))))
    (`MotionWarpingComponent.AddOrUpdateWarpTargetFromLocationAndRotation` :`self` _motionwarpingcomponent :`WarpTargetName` "WarpLocation" :`TargetLocation` _returnvalue_7)
    (`KismetSystemLibrary.DrawDebugSphere` _returnvalue_7 100.0 12 (struct :`R` 1.0 :`G` 1.0 :`B` 1.0 :`A` 1.0) 5.0)
    (else
      (`MotionWarpingComponent.AddOrUpdateWarpTargetFromLocationAndRotation` :`self` _motionwarpingcomponent :`WarpTargetName` "WarpLocation" :`TargetLocation` _returnvalue_5)
      (`KismetSystemLibrary.DrawDebugSphere` _returnvalue_5 100.0 12 (struct :`R` 1.0 :`G` 1.0 :`B` 1.0 :`A` 1.0) 5.0))))

(fn `HandleApplyDamage`
  (params (GameplayEventData :type "GameplayEventData Structure (by ref)"))
  (bind (_eventtag _instigator _target) (break `GameplayEventData` GameplayEventData))
  (`self.K2_ExecuteGameplayCue` (`self.WeaponHitSoundGameplayCueTag`))
  (`self.BP_ApplyEffectSpecHandleToTarget` _target (`self.MakeHeroDamageEffectSpecHandle` "/Game/Asset/_MyAsset/GameEffect/GE_Shared_DealDamage.GE_Shared_DealDamage_C" (`WarriorFunctionLibrary.GetScalableFloatValueAtLevel` (`self.StartDamage`) (`KismetMathLibrary.Conv_IntToDouble` (`self.GetAbilityLevel`))) (struct :`TagName` "Player.SetByCaller.AttackType.Light") 1)
    (:`Successful`
      (`AbilitySystemBlueprintLibrary.SendGameplayEventToActor` _target (struct :`TagName` "Shared.Event.HitReact") (`local.GameplayEventData`))
      (`WarriorFunctionLibrary.AddGameplayTagToActorIfNone` _target (struct :`TagName` "Shared.Status.Burning"))
      (`self.BP_ApplyEffectSpecHandleToTarget` _target (`self.MakeHeroStatusEffectSpecHandle` "/Game/Asset/_MyAsset/GameEffect/GE_Shared_IceDamage.GE_Shared_IceDamage_C" (`WarriorFunctionLibrary.GetScalableFloatValueAtLevel` (`self.BurningDamage`) (`KismetMathLibrary.Conv_IntToDouble` (`self.GetAbilityLevel`))) (struct :`TagName` "Player.SetByCaller.AttackType.Status") (struct :`TagName` "Shared.DamageType.Ice") 0 0 (`WarriorFunctionLibrary.GetScalableFloatValueAtLevel` (`self.BurningDuration`) (`KismetMathLibrary.Conv_IntToDouble` (`self.GetAbilityLevel`))))
        (:`Successful`
          (`self.BP_ApplyGameplayEffectToOwner` "/Game/Asset/_MyAsset/GameEffect/GE_Hero_GainRage.GE_Hero_GainRage_C" (`self.GetAbilityLevel`))
          (return))
        (:`Failed`
          (return))))
    (:`Failed`
      (return))))