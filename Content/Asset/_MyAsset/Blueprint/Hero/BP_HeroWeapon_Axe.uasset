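; BP_HeroWeapon_Axe is the hero's axe weapon, handling equip, unequip and collision toggling.
; Equip and unequip attach it to right-hand or back sockets, with timelines animating the mesh's DissolveAmount material parameter in reverse and forward respectively.
; Registering sets DissolveAmount to 1.
; Collision toggles for the current-equipped-weapon damage type switch the box between query-only and disabled, with a debug print.
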(event `self.BP_OnEquipWeapon`
  (params (TargetMesh :type "SkeletalMeshComponent Object Reference"))
  (`self.K2_AttachToComponent` TargetMesh "AxeRightHandSocket" "SnapToTarget" "SnapToTarget" "KeepWorld")
  (bind (_direction _normalizedfloattrack) (`Timeline|Timeline` :!via `ReverseFromEnd`)
    (:`Update`
      (`MeshComponent.SetScalarParameterValueOnMaterials` (`self.WeaponMeshComponent`) "DissolveAmount" _normalizedfloattrack))))

(event `self.BP_ToggleCurrentEquippedWeaponCollision`
  (params (bShouldEnable :type Boolean) (ToggleDamageType :type "EToggleDamageType Enum" :default "CurrentEquippedWeapon"))
  (if (`|EnumEquality` ToggleDamageType "CurrentEquippedWeapon")
    (`PrimitiveComponent.SetCollisionEnabled` (`self.WeaponCollisionBox`) (select `bool` bShouldEnable :`false` "NoCollision" :`true` "QueryOnly" :!type "ECollisionEnabled Enum"))
    (`KismetSystemLibrary.PrintString` "ToggleAxe")))

(event `self.BP_OnWeaponRegister`
  (`MeshComponent.SetScalarParameterValueOnMaterials` (`self.WeaponMeshComponent`) "DissolveAmount" 1.0))

(event `self.BP_OnUnequip`
  (params (TargetMesh :type "SkeletalMeshComponent Object Reference"))
  (`self.K2_AttachToComponent` TargetMesh "AxeBackSocket" "SnapToTarget" "KeepRelative" "KeepWorld")
  (bind (_direction _normalizedfloattrack) (`Timeline|Timeline_0` :!via `PlayFromStart`)
    (:`Update`
      (`MeshComponent.SetScalarParameterValueOnMaterials` (`self.WeaponMeshComponent`) "DissolveAmount" _normalizedfloattrack))))

(fn `UserConstructionScript`
  (`parent.UserConstructionScript`))