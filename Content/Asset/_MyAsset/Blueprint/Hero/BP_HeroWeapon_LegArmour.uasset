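; Hero weapon Blueprint for an armour set worn on both arms and legs, with per-limb collision for attacks.
; Equipping attaches four meshes to skeletal mesh sockets and reverses a dissolve timeline to reveal them.
; Unequipping plays the dissolve, then detaches and hides the actor.
; A damage-type selection toggles query-only collision on the matching limb, and overlap delegates for three limb colliders are bound inside ActorBeginOverlap.
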(event `self.BP_OnUnequip`
  (params (TargetMesh :type "SkeletalMeshComponent Object Reference"))
  (bind (_direction _normalizedfloattrack) (`Timeline|Timeline` :!via `PlayFromStart`)
    (:`Update`
      (`MeshComponent.SetScalarParameterValueOnMaterials` (`self.WeaponMeshComponent`) "DissolveAmount" _normalizedfloattrack)
      (`MeshComponent.SetScalarParameterValueOnMaterials` (`self.RightArm`) "DissolveAmount" _normalizedfloattrack)
      (`MeshComponent.SetScalarParameterValueOnMaterials` (`self.LeftLeg`) "DissolveAmount" _normalizedfloattrack)
      (`MeshComponent.SetScalarParameterValueOnMaterials` (`self.RightLeg`) "DissolveAmount" _normalizedfloattrack))
    (:`Finished`
      (`self.DetachFromSkeletalMesh` TargetMesh)
      (`self.SetActorHiddenInGame` true))))

(event `self.BP_OnEquipWeapon`
  (params (TargetMesh :type "SkeletalMeshComponent Object Reference"))
  (`self.AttachToSkeletal Mesh` TargetMesh "SnapToTarget")
  (`self.SetActorHiddenInGame` false)
  (bind (_direction _normalizedfloattrack) (`Timeline|Timeline_0` :!via `ReverseFromEnd`)
    (:`Update`
      (`MeshComponent.SetScalarParameterValueOnMaterials` (`self.WeaponMeshComponent`) "DissolveAmount" _normalizedfloattrack)
      (`MeshComponent.SetScalarParameterValueOnMaterials` (`self.RightArm`) "DissolveAmount" _normalizedfloattrack)
      (`MeshComponent.SetScalarParameterValueOnMaterials` (`self.LeftLeg`) "DissolveAmount" _normalizedfloattrack)
      (`MeshComponent.SetScalarParameterValueOnMaterials` (`self.RightLeg`) "DissolveAmount" _normalizedfloattrack))))

(event `self.BP_OnWeaponRegister`
  (`MeshComponent.SetScalarParameterValueOnMaterials` (`self.WeaponMeshComponent`) "DissolveAmount" 1.0)
  (`MeshComponent.SetScalarParameterValueOnMaterials` (`self.RightArm`) "DissolveAmount" 1.0)
  (`MeshComponent.SetScalarParameterValueOnMaterials` (`self.LeftLeg`) "DissolveAmount" 1.0)
  (`MeshComponent.SetScalarParameterValueOnMaterials` (`self.RightLeg`) "DissolveAmount" 1.0))

(event `self.BP_ToggleCurrentEquippedWeaponCollision`
  (params (bShouldEnable :type Boolean) (ToggleDamageType :type "EToggleDamageType Enum" :default "CurrentEquippedWeapon"))
  (bind _weaponcollisionbox (`self.WeaponCollisionBox`))
  (`PrimitiveComponent.SetCollisionEnabled` (select `EToggleDamageType` ToggleDamageType :`CurrentEquippedWeapon` _weaponcollisionbox :`LeftHand` _weaponcollisionbox :`RightHand` (`self.RightArmLegCollision`) :`LeftLeg` (`self.LeftLegCollision`) :`RightLeg` (`self.RightLegCollision`) :!type "PrimitiveComponent Object Reference") (select `bool` bShouldEnable :`false` "NoCollision" :`true` "QueryOnly" :!type "ECollisionEnabled Enum")))

(event `self.ReceiveActorBeginOverlap`
  (params (OtherActor :type "Actor Object Reference"))
  (bind _rightarmlegcollision (`self.RightArmLegCollision`))
  (`parent.ReceiveActorBeginOverlap` OtherActor)
  (add `PrimitiveComponent.OnComponentBeginOverlap` _rightarmlegcollision (`|CreateDelegate` :!event `HandleBeginOverlap`))
  (add `PrimitiveComponent.OnComponentBeginOverlap` (`self.LeftLegCollision`) (`|CreateDelegate` :!event `HandleBeginOverlap`))
  (add `PrimitiveComponent.OnComponentBeginOverlap` (`self.RightLegCollision`) (`|CreateDelegate` :!event `HandleBeginOverlap`))
  (add `PrimitiveComponent.OnComponentEndOverlap` _rightarmlegcollision (`|CreateDelegate` :!event `HandleEndOverlap`)))

(fn `AttachToSkeletal Mesh`
  (params (Mesh :type "SkeletalMeshComponent Object Reference") (ScaleRule :type "EAttachmentRule Enum" :default "KeepRelative"))
  (`SceneComponent.K2_AttachToComponent` (`self.LeftLeg`) Mesh "Armour_LL" "SnapToTarget" "KeepRelative" ScaleRule true)
  (`SceneComponent.K2_AttachToComponent` (`self.RightLeg`) Mesh "Armour_RL" "SnapToTarget" "KeepRelative" ScaleRule true)
  (`SceneComponent.K2_AttachToComponent` (`self.RightArm`) Mesh "Armour_RH" "SnapToTarget" "KeepRelative" ScaleRule true)
  (`SceneComponent.K2_AttachToComponent` (`self.WeaponMeshComponent`) Mesh "Armour_LH" "SnapToTarget" "KeepRelative" ScaleRule true))

(fn `DetachFromSkeletalMesh`
  (params (Mesh :type "SkeletalMeshComponent Object Reference"))
  (`SceneComponent.K2_DetachFromComponent` (`self.LeftLeg`) "KeepRelative" "KeepRelative" "KeepRelative" true)
  (`SceneComponent.K2_DetachFromComponent` (`self.RightLeg`) "KeepRelative" "KeepRelative" "KeepRelative" true)
  (`SceneComponent.K2_DetachFromComponent` (`self.RightArm`) "KeepRelative" "KeepRelative" "KeepRelative" true)
  (`SceneComponent.K2_DetachFromComponent` (`self.WeaponMeshComponent`) "KeepRelative" "KeepRelative" "KeepRelative" true)
  (`SceneComponent.K2_AttachToComponent` (`self.RightArm`) (`self.WeaponMeshComponent`) "None" "KeepRelative" "KeepRelative" "KeepRelative" true))

(fn `UserConstructionScript`
  (`parent.UserConstructionScript`))